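; Sweeper is an actor that travels along a spline and destroys any AutoBotVehicle that overlaps its box.
; When ActiveKiller is set, BeginPlay starts a timeline that lerps distance along TrackRef's spline, setting the actor's world location and rotation.
; ReverseDirection runs the timeline from the end, and its play rate is the inverse of Speed, so higher Speed values mean slower travel.
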(event OnComponentBeginOverlap(Box)
  (params (OverlappedComponent :type Primitive%20Component%20Object%20Reference) (OtherActor :type Actor%20Object%20Reference) (OtherComp :type Primitive%20Component%20Object%20Reference) (OtherBodyIndex :type Integer) (bFromSweep :type Boolean) (SweepResult :type Hit%20Result%20Structure%20%28by%20ref%29))
  (bind _asauto_bot_vehicle (Utilities|Casting|CastToAutoBotVehicle OtherActor))
  (Actor|DestroyActor _asauto_bot_vehicle))

(event Custom|MoveKiller
  (bind _trackref (Variables|Default|GetTrackRef))
  (bind _spline (Variables|/Game/Blueprints/BP_Spline_V2.BP_Spline_V2_C|GetSpline _trackref))
  (Components|Timeline|SetPlayRate (Variables|Default|GetTimeline_0) (/ 1.0 (Variables|Default|Getspeed)))
  (Components|Timeline|SetNewTime (Variables|Default|GetTimeline_0) 0.0)
  (if (Variables|Default|GetReverseDirection)
    (bind _alpha (Timeline|Timeline_0 ReverseFromEnd)
      (:Update
        (Transformation|SetActorLocationAndRotation (Spline|GetLocationatDistanceAlongSpline _spline (Math|Float|Lerp 0.0 (Spline|GetSplineLength (Variables|/Game/Blueprints/BP_Spline_V2.BP_Spline_V2_C|GetSpline (Variables|Default|GetTrackRef))) _alpha) "World") (Spline|GetRotationatDistanceAlongSpline _spline (Math|Float|Lerp 0.0 (Spline|GetSplineLength (Variables|/Game/Blueprints/BP_Spline_V2.BP_Spline_V2_C|GetSpline (Variables|Default|GetTrackRef))) _alpha) "World"))))
    (else
      (Timeline|Timeline_0 PlayFromStart))))

(event EventBeginPlay
  (if (Variables|Default|GetActiveKiller)
    (CallFunction|MoveKiller)))

(fn ConstructionScript)