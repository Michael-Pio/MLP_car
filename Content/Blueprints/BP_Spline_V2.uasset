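; Spline actor that populates its path with meshes from a StaticMeshes list when constructed.
; Base entries become chained spline mesh segments that bend along the curve, with tangents clamped to the ScaleX-scaled section length.
; Other entries become instanced static meshes spaced along the spline, each rotated toward the previous point and shifted by an offset.
; IsEditMode turns generated collision off, otherwise query-only; the Visiblity flag also shortens the segment loop.
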(event EventBeginPlay)

(event Collision|EventActorBeginOverlap
  (params (OtherActor :type Actor%20Object%20Reference)))

(event EventTick
  (params (DeltaSeconds :type Float%20%28single-precision%29)))

(fn ConstructionScript
  (Utilities|FlowControl|Sequence
    (:then_0
      (if (Variables|Default|GetIsEditMode)
        (LocalVariables|SetCollisionPreset "NoCollision")
        (else
          (LocalVariables|SetCollisionPreset "QueryOnly"))))
    (:then_1
      (for _array_element (Variables|Default|GetStaticMeshes)
        (if (.IsThatBase (Utilities|Struct|BreakSplineObject _array_element))
          (bind _output_get (LocalVariables|SetupdatedSectionLength (* (.SectionLength (Utilities|Struct|BreakSplineObject _array_element)) (Variables|Default|GetScaleX))))
          (for _index (range 0 (CallFunction|GetNumOfSegments (.visiblity (Utilities|Struct|BreakSplineObject _array_element)) _output_get))
            (bind _returnvalue (AddComponent|AddSplineMeshComponent false))
            (Components|StaticMesh|SetStaticMesh _returnvalue (.PopulatingMesh (Utilities|Struct|BreakSplineObject _array_element)))
            (SplineMesh|SetForwardAxis _returnvalue (.ForwardAxis (Utilities|Struct|BreakSplineObject _array_element)) true)
            (SplineMesh|SetStartandEnd _returnvalue (.StartPosition (CallFunction|GetStartEndPositionTangent (LocalVariables|GetupdatedSectionLength) _index)) (.StartTangent (CallFunction|GetStartEndPositionTangent (LocalVariables|GetupdatedSectionLength) _index)) (.EndPosition (CallFunction|GetStartEndPositionTangent (LocalVariables|GetupdatedSectionLength) _index)) (.EndTangent (CallFunction|GetStartEndPositionTangent (LocalVariables|GetupdatedSectionLength) _index)) true :!class /Script/Engine.SplineMeshComponent)
            (Collision|SetCollisionEnabled _returnvalue (LocalVariables|GetCollisionPreset))
            (Rendering|SetVisibility _returnvalue (.visiblity (Utilities|Struct|BreakSplineObject _array_element)) false))
          (else
            (bind _returnvalue_2 (AddComponent|AddInstancedStaticMeshComponent false))
            (Variables|Default|SetInstancedStaticMesh _returnvalue_2)
            (Components|StaticMesh|SetStaticMesh _returnvalue_2 (.PopulatingMesh (Utilities|Struct|BreakSplineObject _array_element)))
            (LocalVariables|SetupdatedSectionLength (.x (+ (.Offset (Utilities|Struct|BreakSplineObject _array_element)) (Math|Vector|MakeVector (.SectionLength (Utilities|Struct|BreakSplineObject _array_element)) 0.0 0.0))))
            (for _index_2 (range 1 (Math|Float|Floor (/ (Spline|GetSplineLength (Variables|Default|GetSpline)) (LocalVariables|GetupdatedSectionLength))))
              (Components|InstancedStaticMesh|AddInstance _returnvalue_2 (Math|Transform|MakeTransform (CallFunction|GetLocationOfSectionbyIndex _index_2 (LocalVariables|GetupdatedSectionLength)) (Math|Conversions|RotationFromXVector (- (CallFunction|GetLocationOfSectionbyIndex (- _index_2 1) (LocalVariables|GetupdatedSectionLength)) (CallFunction|GetLocationOfSectionbyIndex _index_2 (LocalVariables|GetupdatedSectionLength))))))
              (Rendering|SetVisibility _returnvalue_2 (.visiblity (Utilities|Struct|BreakSplineObject _array_element)) true)
              (Collision|SetCollisionEnabled _returnvalue_2 (LocalVariables|GetCollisionPreset))
              (Transformation|AddLocalOffset (Variables|Default|GetInstancedStaticMesh) (.Offset (Utilities|Struct|BreakSplineObject _array_element)) false true))))))))

(fn GetStartEndPositionTangent
  (params (updatedSectionLength :type Float%20%28single-precision%29) (index :type Integer))
  (bind _returnvalue (* index updatedSectionLength))
  (bind _returnvalue_2 (+ index 1))
  (bind _spline (Variables|Default|GetSpline))
  (bind _spline_2 (Variables|Default|GetSpline))
  (bind _returnvalue_3 (* _returnvalue_2 updatedSectionLength))
  (return (Spline|GetLocationatDistanceAlongSpline _spline_2 _returnvalue "Local") (Math|Vector|ClampVectorSize (Spline|GetTangentatDistanceAlongSpline _spline_2 _returnvalue "Local") 0.0 updatedSectionLength) (Spline|GetLocationatDistanceAlongSpline _spline _returnvalue_3 "Local") (Math|Vector|ClampVectorSize (Spline|GetTangentatDistanceAlongSpline _spline _returnvalue_3 "Local") 0.0 updatedSectionLength)))

(fn GetNumOfSegments
  (params (mustBeFullLengthMeshs :type Boolean) (UpdatedSectionLength :type Float%20%28single-precision%29))
  (bind _spline (Variables|Default|GetSpline))
  (bind _returnvalue (Spline|GetSplineLength _spline))
  (bind _returnvalue_2 (/ _returnvalue UpdatedSectionLength))
  (bind _returnvalue_3 (Math|Float|Truncate _returnvalue_2))
  (if mustBeFullLengthMeshs
    (return (- _returnvalue_3 1))
    (else
      (return _returnvalue_3))))

(fn GetLocationOfSectionbyIndex
  (params (Index :type Integer) (sectionLength :type Float%20%28single-precision%29))
  (return (Spline|GetLocationatDistanceAlongSpline (Variables|Default|GetSpline) (* Index sectionLength) "Local")))