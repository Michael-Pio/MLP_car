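; Spline track actor that populates its spline with repeated static meshes at construction time.
; Each StaicMeshes entry creates an instanced static mesh component with its own mesh, visibility, collision and offset.
; Instances are spaced by mesh X bounds plus X offset and oriented along the line from the current to the previous spline point.
; The local offset moves the whole component on every loop pass, so it accumulates with instance count.
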(event OnComponentEndOverlap(Spline)
  (params (OverlappedComponent :type Primitive%20Component%20Object%20Reference) (OtherActor :type Actor%20Object%20Reference) (OtherComp :type Primitive%20Component%20Object%20Reference) (OtherBodyIndex :type Integer)))

(event EventBeginPlay)

(event Collision|EventActorBeginOverlap
  (params (OtherActor :type Actor%20Object%20Reference)))

(event EventTick
  (params (DeltaSeconds :type Float%20%28single-precision%29)))

(fn ConstructionScript
  (for _array_element (Variables|Default|GetStaicMeshes)
    (Utilities|FlowControl|Sequence
      (:then_0
        (LocalVariables|Setselected_mesh (.PopulatingMesh (Utilities|Struct|BreakSplineObject _array_element)))
        (LocalVariables|Setoffset (.Offset (Utilities|Struct|BreakSplineObject _array_element)))
        (LocalVariables|SetMeshVisiblity (.visiblity (Utilities|Struct|BreakSplineObject _array_element)))
        (LocalVariables|SetCollision (.Collision (Utilities|Struct|BreakSplineObject _array_element))))
      (:then_1
        (bind _returnvalue (AddComponent|AddInstancedStaticMeshComponent false))
        (Variables|Default|SetInstancedStaticMesh _returnvalue)
        (Components|StaticMesh|SetStaticMesh (Variables|Default|GetInstancedStaticMesh) (LocalVariables|Getselected_mesh))
        (LocalVariables|Setspacing (CallFunction|GetSpacingforStaticMesh (LocalVariables|Getselected_mesh) (.x (LocalVariables|Getoffset))))
        (for _index (range 0 (Math|Float|Floor (/ (Spline|GetSplineLength (Variables|Default|GetSpline)) (LocalVariables|Getspacing))))
          (Components|InstancedStaticMesh|AddInstance (Variables|Default|GetInstancedStaticMesh) (Math|Transform|MakeTransform (CallFunction|GetLocationbyIndex _index (LocalVariables|Getspacing)) (Math|Conversions|RotationFromXVector (- (CallFunction|GetLocationbyIndex (- _index 1) (LocalVariables|Getspacing)) (CallFunction|GetLocationbyIndex _index (LocalVariables|Getspacing))))))
          (Rendering|SetVisibility (Variables|Default|GetInstancedStaticMesh) (LocalVariables|GetMeshVisiblity) true)
          (Collision|SetCollisionEnabled (Variables|Default|GetInstancedStaticMesh) (LocalVariables|GetCollision))
          (Transformation|AddLocalOffset (Variables|Default|GetInstancedStaticMesh) (Math|Vector|MakeVector (.x (LocalVariables|Getoffset)) (.y (LocalVariables|Getoffset)) (.z (LocalVariables|Getoffset))) false true))))))

(fn GetLocationbyIndex
  (params (A :type Integer) (Spacing :type Float%20%28single-precision%29))
  (return (Spline|GetLocationatDistanceAlongSpline (Variables|Default|GetSpline) (* A Spacing) "Local")))

(fn GetSpacingforStaticMesh
  (params (Mesh :type Static%20Mesh%20Object%20Reference) (Offset :type Float%20%28single-precision%29))
  (bind _returnvalue (StaticMesh|GetBoundingBox Mesh))
  (bind (_min _max) (Utilities|Struct|BreakBox _returnvalue))
  (return (+ (.x (- _max _min)) Offset)))