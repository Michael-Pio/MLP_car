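; MLP_SpectatorPawnBP is a spectator pawn that adds on-screen UI and adjustable movement speed.
; On BeginPlay it creates a HUD widget, which the F key shows or hides through a Visible flag.
; Tab creates a new Pause_MENU widget and adds it to the viewport on each press.
; The mouse wheel raises or lowers the FloatingPawnMovement MaxSpeed by a SpeedDiff step, with no clamping.
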(event EventBeginPlay
  (bind _returnvalue (UserInterface|CreateWidget "/Game/UI_BP/HUD.HUD_C"))
  (UserInterface|Viewport|AddtoViewport _returnvalue 0))

(event Input|KeyboardEvents|F
  (params (Key :type Key%20Structure :default "None"))
  (:Pressed
    (if (Variables|Default|GetVisible)
      (Variables|Default|SetVisible false)
      (Widget|SetVisibility (stale EventBeginPlay _returnvalue) "Hidden")
      (else
        (Variables|Default|SetVisible true)
        (Widget|SetVisibility (stale EventBeginPlay _returnvalue) "Visible")))))

(event Input|KeyboardEvents|Tab
  (params (Key :type Key%20Structure :default "None"))
  (:Pressed
    (bind _returnvalue (UserInterface|CreateWidget "/Game/UI_BP/Pause_MENU.Pause_MENU_C"))
    (UserInterface|Viewport|AddtoViewport _returnvalue 0)))

(event Input|MouseEvents|MouseWheelUp
  (params (Key :type Key%20Structure :default "None"))
  (:Pressed
    (bind _asfloating_pawn_movement (Utilities|Casting|CastToFloatingPawnMovement (Variables|Default|GetMovementComponent)))
    (Variables|/Script/Engine.FloatingPawnMovement|SetMaxSpeed _asfloating_pawn_movement (+ (Class|MovementComponent|GetMaxSpeed _asfloating_pawn_movement) (Variables|Default|GetSpeedDiff)))))

(event Input|MouseEvents|MouseWheelDown
  (params (Key :type Key%20Structure :default "None"))
  (:Pressed
    (bind _asfloating_pawn_movement (Utilities|Casting|CastToFloatingPawnMovement (Variables|Default|GetMovementComponent)))
    (Variables|/Script/Engine.FloatingPawnMovement|SetMaxSpeed _asfloating_pawn_movement (- (Class|MovementComponent|GetMaxSpeed _asfloating_pawn_movement) (Variables|Default|GetSpeedDiff)))))

(fn ConstructionScript)